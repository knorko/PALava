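; Actor that acts as a paintable flowmap surface, with events to paint, erase and reset flow and to toggle the overlaid surface plane.
; Construction creates brush and eraser dynamic materials and applies an optional mesh to both planes.
; Paint and erase convert world positions into plane-relative UVs, then draw those materials into RT_Flowmap.
; Erasing first draws a copy material into a swap render target; reset clears both targets.
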(event `self.ReceiveBeginPlay`)

(event `CE_Draw`
  (params (Position :type "Vector Structure") (Velocity :type "Vector Structure") (Radius :type "Float (double-precision)"))
  (bind _brushmaterial (`self.BrushMaterial`))
  (bind _plane (`self.Plane`))
  (bind (_origin _boxextent _sphereradius) (`KismetSystemLibrary.GetComponentBounds` _plane))
  (bind _returnvalue_x (`KismetMathLibrary.BreakVector` (`SceneComponent.K2_GetComponentScale` _plane)))
  ;[1 1 1] Paint
  (`MaterialInstanceDynamic.SetVectorParameterValue` _brushmaterial "Position" (`KismetMathLibrary.Conv_VectorToLinearColor` (+ (/ (`KismetMathLibrary.InverseTransformLocation` (`self.GetTransform`) Position) (/ (* (.x _boxextent) 2.0) _returnvalue_x)) 0.5)))
  (`MaterialInstanceDynamic.SetVectorParameterValue` _brushmaterial "Velocity" (`KismetMathLibrary.Conv_VectorToLinearColor` Velocity))
  (`MaterialInstanceDynamic.SetScalarParameterValue` _brushmaterial "Radius" (/ Radius (* _sphereradius 0.0001)))
  (`KismetRenderingLibrary.DrawMaterialToRenderTarget` "/Game/PA/Textures/RenderTarget/RT_Flowmap.RT_Flowmap" _brushmaterial))

(event `CE_ToggleSurfaceMaterial`
  (bind _plane1 (`self.Plane1`))
  ;[1 1 1] Hide Surface Plane
  (`SceneComponent.SetHiddenInGame` _plane1 (not (`SceneComponent.bHiddenInGame` _plane1)) false))

(event `CE_ResetFlowmap`
  ;[1 1 1] Reset Flowmap
  (`KismetRenderingLibrary.ClearRenderTarget2D` "/Game/PA/Textures/RenderTarget/RT_Flowmap.RT_Flowmap" (make `LinearColor` 1.0 1.0))
  (`KismetRenderingLibrary.ClearRenderTarget2D` "/Game/PA/Textures/RenderTarget/RT_Flowmap_Swap.RT_Flowmap_Swap" (make `LinearColor` 1.0 1.0)))

(event `CE_Erase`
  (params (Position :type "Vector Structure") (Radius :type "Float (double-precision)"))
  (bind _plane (`self.Plane`))
  (bind _erasermaterial (`self.EraserMaterial`))
  (bind _returnvalue_x (`KismetMathLibrary.BreakVector` (`SceneComponent.K2_GetComponentScale` _plane)))
  ;[1 1 1] Erase
  (`KismetRenderingLibrary.DrawMaterialToRenderTarget` "/Game/PA/Textures/RenderTarget/RT_Flowmap_Swap.RT_Flowmap_Swap" "/Game/PA/Materials/Framework/M_CopyRT.M_CopyRT")
  (`MaterialInstanceDynamic.SetVectorParameterValue` _erasermaterial "Position" (`KismetMathLibrary.Conv_VectorToLinearColor` (+ (/ (`KismetMathLibrary.InverseTransformLocation` (`self.GetTransform`) Position) (/ (* (.x (`.BoxExtent` (`KismetSystemLibrary.GetComponentBounds` _plane))) 2.0) _returnvalue_x)) 0.5)))
  (`MaterialInstanceDynamic.SetVectorParameterValue` _erasermaterial "Velocity" (make `LinearColor` 0.0))
  (`MaterialInstanceDynamic.SetScalarParameterValue` _erasermaterial "Radius" Radius)
  (`KismetRenderingLibrary.DrawMaterialToRenderTarget` "/Game/PA/Textures/RenderTarget/RT_Flowmap.RT_Flowmap" _erasermaterial))

(fn `UserConstructionScript`
  (bind _meshasset (`self.MeshAsset`))
  (`|ExecutionSequence`
    (:`then_0`
      (bind _returnvalue (`KismetMaterialLibrary.CreateDynamicMaterialInstance` "/Game/PA/Materials/Framework/M_Brush_Paint.M_Brush_Paint"))
      (set `self.BrushMaterial` _returnvalue))
    (:`then_1`
      (bind _returnvalue_2 (`KismetMaterialLibrary.CreateDynamicMaterialInstance` "/Game/PA/Materials/Framework/M_Brush_Erase.M_Brush_Erase"))
      (set `self.EraserMaterial` _returnvalue_2))
    (:`then_2`
      (`/Engine/EditorBlueprintResources/StandardMacros.IsValid` _meshasset
        (:`Is Valid`
          (`StaticMeshComponent.SetStaticMesh` (`self.Plane`) _meshasset)
          (`StaticMeshComponent.SetStaticMesh` (`self.Plane1`) _meshasset))))))