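; Player character for painting flowmaps onto BP_FlowmapPlane actors with the mouse.
; Each tick traces under the cursor, moves a sphere cursor to the hit and derives brush radius from its scale and stroke velocity from hit movement.
; Left mouse paints velocity and Alt-click erases, with look input suspended during strokes.
; The wheel resizes the brush, while hotkeys toggle the surface material, export or reset the flowmap.
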(event `self.ReceiveBeginPlay`
  (bind _returnvalue (`GameplayStatics.GetPlayerController` 0))
  (`|ExecutionSequence`
    (:`then_0`
      (`|ExecutionSequence`
        (:`then_0`
          (set `self.PitchScale_Init` (`PlayerController.InputPitchScale` _returnvalue)))
        (:`then_1`
          (set `self.RollScale_Init` (`PlayerController.InputRollScale` _returnvalue)))
        (:`then_2`
          (set `self.YawScale_Init` (`PlayerController.InputYawScale` _returnvalue)))))
    (:`then_1`
      (set `PlayerController.bShowMouseCursor` true (`GameplayStatics.GetPlayerController` 0)))))

(event `self.ReceiveTick`
  (params (DeltaSeconds :type "Float (single-precision)"))
  (bind _returnvalue (`GameplayStatics.GetPlayerController` 0))
  (bind _returnvalue_2 (`GameplayStatics.GetPlayerController` 0))
  (bind _flowmapplane (`self.FlowmapPlane`))
  (bind _flowmapplane_2 (`self.FlowmapPlane`))
  (bind _returnvalue_x (`KismetMathLibrary.BreakVector` (`SceneComponent.K2_GetComponentScale` (`self.Sphere`))))
  (bind _returnvalue_x_2 (`KismetMathLibrary.BreakVector` (`SceneComponent.K2_GetComponentScale` (`/Game/PA/Blueprints/BP_FlowmapPlane.Plane` _flowmapplane))))
  ;[1 1 1] Tick
  (`|ExecutionSequence`
    (:`then_0`
      (`self.fTraceUnderMouse`))
    (:`then_1`
      (`self.fUpdateSphereLocation`))
    (:`then_2`
      (`/Engine/EditorBlueprintResources/StandardMacros.IsValid` _flowmapplane
        (:`Is Valid`
          (set `self.BrushRadius` (/ (/ (* _returnvalue_x 100.0) 2.0) _returnvalue_x_2)))))
    (:`then_3`
      (if (`self.bLeftMouseDown`)
        (`|ExecutionSequence`
          (:`then_0`
            (`/Engine/EditorBlueprintResources/StandardMacros.DoOnce` false :!label _label
              (:`Completed`
                (`|ExecutionSequence`
                  (:`then_0`
                    (set `PlayerController.InputRollScale` 0.0 _returnvalue_2))
                  (:`then_1`
                    (set `PlayerController.InputPitchScale` 0.0 _returnvalue_2))
                  (:`then_2`
                    (set `PlayerController.InputYawScale` 0.0 _returnvalue_2))))))
          (:`then_1`
            (if (not (`self.bControlModifier`))
              (bind _output_get (set `self.Velocity` (* (`self.MouseVelocity`) (`self.Intensity`))))
              (`/Engine/EditorBlueprintResources/StandardMacros.IsValid` _flowmapplane_2
                (:`Is Valid`
                  (`/Game/PA/Blueprints/BP_FlowmapPlane.CE_Draw` _flowmapplane_2 (`self.Position`) _output_get (`self.BrushRadius`))))
              (else
                (`/Game/PA/Blueprints/BP_FlowmapPlane.CE_Erase` _flowmapplane_2 (`self.Position`) (`self.BrushRadius`)))))
          (:`then_2`
            (goto _label_2 :!via `Reset`)))
        (else
          (`/Engine/EditorBlueprintResources/StandardMacros.DoOnce` false :!label _label_2
            (:`Completed`
              (`|ExecutionSequence`
                (:`then_0`
                  (goto _label :!via `Reset`))
                (:`then_1`
                  (set `PlayerController.InputRollScale` (`self.RollScale_Init`) _returnvalue))
                (:`then_2`
                  (set `PlayerController.InputPitchScale` (`self.PitchScale_Init`) _returnvalue))
                (:`then_3`
                  (set `PlayerController.InputYawScale` (`self.YawScale_Init`) _returnvalue))))))))))

(event `Key|H`
  (params (Key :type "Key Structure"))
  (bind _flowmapplane (`self.FlowmapPlane`))
  ;[1 1 1] Hide Surface Material
  (:`Pressed`
    (`/Engine/EditorBlueprintResources/StandardMacros.IsValid` _flowmapplane
      (:`Is Valid`
        (`/Game/PA/Blueprints/BP_FlowmapPlane.CE_ToggleSurfaceMaterial` _flowmapplane)))))

(event `Key|One`
  (params (Key :type "Key Structure"))
  (bind _flowmapplane (`self.FlowmapPlane`))
  (:`Pressed`
    (`/Engine/EditorBlueprintResources/StandardMacros.IsValid` _flowmapplane
      (:`Is Valid`
        (`/Game/PA/Blueprints/BP_FlowmapPlane.CE_ExportFlowmap` _flowmapplane)))))

(event `Key|R`
  (params (Key :type "Key Structure"))
  (bind _flowmapplane (`self.FlowmapPlane`))
  ;[1 1 1] ResetFlowmap
  (:`Pressed`
    (`/Engine/EditorBlueprintResources/StandardMacros.IsValid` _flowmapplane
      (:`Is Valid`
        (`/Game/PA/Blueprints/BP_FlowmapPlane.CE_ResetFlowmap` _flowmapplane)))))

(event `Key|LeftMouseButton`
  (params (Key :type "Key Structure"))
  ;[1 1 1] Paint
  (:`Pressed`
    (set `self.bLeftMouseDown` true))
  (:`Released`
    (set `self.bLeftMouseDown` false)))

(event `Key|MouseScrollUp`
  (params (Key :type "Key Structure"))
  (bind _sphere (`self.Sphere`))
  (bind _returnvalue_x (`KismetMathLibrary.BreakVector` (+ (`SceneComponent.K2_GetComponentScale` _sphere) (1.0 1.0 1.0))))
  (bind _returnvalue (`KismetMathLibrary.FClamp` _returnvalue_x 0.0 1000.0))
  ;[1 1 1] ScaleBrushSize
  (:`Pressed`
    (`SceneComponent.SetWorldScale3D` _sphere (`KismetMathLibrary.MakeVector` _returnvalue _returnvalue _returnvalue))))

(event `Key|Alt+LeftMouseButton`
  (params (Key :type "Key Structure"))
  ;[1 1 1] Paint
  (:`Pressed`
    (set `self.bLeftMouseDown` true)
    (set `self.bControlModifier` true))
  (:`Released`
    (set `self.bLeftMouseDown` false)
    (set `self.bControlModifier` false)))

(event `Key|MouseScrollDown`
  (params (Key :type "Key Structure"))
  (bind _sphere (`self.Sphere`))
  (bind _returnvalue_x (`KismetMathLibrary.BreakVector` (- (`SceneComponent.K2_GetComponentScale` _sphere) (1.0 1.0 1.0))))
  (bind _returnvalue (`KismetMathLibrary.FClamp` _returnvalue_x 0.0 1000.0))
  ;[1 1 1] ScaleBrushSize
  (:`Pressed`
    (`SceneComponent.SetWorldScale3D` _sphere (`KismetMathLibrary.MakeVector` _returnvalue _returnvalue _returnvalue))))

(fn `FAdjustFlightSpeedToHeight`
  (bind _returnvalue (`self.K2_GetActorLocation`))
  (bind _outhit (`KismetSystemLibrary.LineTraceSingleForObjects` _returnvalue (- _returnvalue (0.0 0.0 10000.0)) (`|MakeArray` "ObjectTypeQuery1" :!type "EObjectTypeQuery Enum")))
  (`KismetSystemLibrary.PrintString` (`KismetStringLibrary.Conv_DoubleToString` (`.Distance` (`GameplayStatics.BreakHitResult` _outhit))) true true (struct :`G` 0.66 :`B` 1.0 :`A` 1.0) 0.0)
  (`KismetSystemLibrary.PrintString` "Hello" true true (struct :`G` 0.66 :`B` 1.0 :`A` 1.0) 0.0))

(fn `fTraceUnderMouse`
  (bind (_hitresult _returnvalue) (`PlayerController.GetHitResultUnderCursorForObjects` (`GameplayStatics.GetPlayerController` 0) (`|MakeArray` "ObjectTypeQuery7" :!type "EObjectTypeQuery Enum") true))
  (bind (_bblockinghit _binitialoverlap _time _distance _location _impactpoint _normal _impactnormal _physmat _hitactor) (`GameplayStatics.BreakHitResult` _hitresult))
  (if _returnvalue
    (`|ExecutionSequence`
      (:`then_0`
        (set `self.MouseVelocity` (- _location (`self.Position`))))
      (:`then_1`
        (set `self.Position` _location))
      (:`then_2`
        (bind _asbp_flowmap_plane (cast `/Game/PA/Blueprints/BP_FlowmapPlane` _hitactor))
        (set `self.FlowmapPlane` _asbp_flowmap_plane))
      (:`then_3`
        (return)))
    (else
      (set `self.FlowmapPlane` null))))

(fn `fUpdateSphereLocation`
  (`SceneComponent.K2_SetWorldLocation` (`self.Sphere`) (`self.Position`) false false))

(fn `UserConstructionScript`
  (bind _returnvalue (`PrimitiveComponent.CreateDynamicMaterialInstance` (`self.Sphere`) 0 "/Game/PA/Materials/Framework/M_Cursor.M_Cursor" "None"))
  (bind _output_get (set `self.CursorMaterial` _returnvalue))
  (bind _output_get_2 (set `self.CursorColorPositive` (make `LinearColor` 0.0 0.13 0.79)))
  (set `self.CursorColorNegative` (make `LinearColor` 0.13 0.79))
  (`MaterialInstanceDynamic.SetVectorParameterValue` _output_get "Color" _output_get_2))