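; BP_Simple is an actor that moves directly toward or away from the player's pawn.
; BeginPlay caches the pawn; each Tick recomputes a normalized direction to it, then adds or subtracts that vector depending on the Engage flag.
; Movement uses SetActorLocation without sweep or delta-time scaling, so speed is one unit per frame.
; The line-of-sight check runs every Tick but is an empty stub, and nothing here sets Engage.
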(event `self.ReceiveBeginPlay`
  (set `self.PlayerPawn` (`Controller.K2_GetPawn` (`GameplayStatics.GetPlayerController` 0))))

(event `self.ReceiveTick`
  (params (DeltaSeconds :type "Float (single-precision)"))
  (`|ExecutionSequence`
    (:`then_0`
      (set `self.MovementVector` (`KismetMathLibrary.Normal` (- (`self.K2_GetActorLocation` (`self.PlayerPawn`)) (`self.K2_GetActorLocation`)))) ; Zuweisung
    )
    (:`then_1`
      (if (`self.Engage`)
        (`self.fMoveTowardsPlayer`) ; Memberfunktion des Blueprint
        (else
          (`self.fMoveAwayFromPlayer`) ; Memberfunktion des Blueprint
        ))
      (`self.fCheckLineOfSight`) ; Memberfunktion des Blueprint
    )))

(fn `fCheckLineOfSight`)

(fn `fMoveAwayFromPlayer`
  (`self.K2_SetActorLocation` (- (`self.K2_GetActorLocation`) (`self.MovementVector`))))

(fn `fMoveTowardsPlayer`
  (`self.K2_SetActorLocation` (+ (`self.K2_GetActorLocation`) (`self.MovementVector`))))

(fn `UserConstructionScript`)